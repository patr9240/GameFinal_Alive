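; Hex door actor that opens when something overlaps it and closes once the overlap ends.
; Begin overlap creates and plays a player for the OpenHexDoor1 level sequence and sets the in-use and open flags.
; Tick polls those flags and, with no overlap, plays the sequence in reverse.
; The flags are never cleared, so the reverse call repeats each tick, and the trailing delay leads nowhere.
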(event Collision|EventActorBeginOverlap
  (params (OtherActor :type Actor%20Object%20Reference))
  ;[1 1 1] open hex door 1
  (Variables|Default|SetOverlap true)
  (if (not false)
    (Variables|Default|SetdoorInUse true)
    (bind _returnvalue (Sequencer|Player|CreateLevelSequencePlayer "/Game/Cinematics/OpenHexDoor1.OpenHexDoor1"))
    (Audio|Components|Audio|Play _returnvalue)
    (Variables|Default|SetdoorOpen true)))

(event Collision|EventActorEndOverlap
  (params (OtherActor :type Actor%20Object%20Reference))
  ;[1 1 1] Close hex door 1
  (bind _output_get (Variables|Default|SetOverlap false)))

(event EventTick
  (params (DeltaSeconds :type Float%20%28single-precision%29))
  ;[1 1 1] Close hex door 1
  (if (Math|Boolean|ANDBoolean (not (stale Collision|EventActorEndOverlap _output_get)) (Variables|Default|GetdoorInUse) (Variables|Default|GetdoorOpen))
    (Class|LevelSequencePlayer|PlayReverse (stale Collision|EventActorBeginOverlap _returnvalue))
    (Utilities|FlowControl|Delay 2.3)))

(fn ConstructionScript)